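; BP_PlayerDronePawn is the player's drone pawn Blueprint, connecting health, ammo and death events to the on-screen HUD.
; On BeginPlay it clears all widgets, creates UI_HUD for player 0 and seeds it with the ShootingComponent's current ammo.
; Ammo and health change events push new values to the HUD, and OnDeath reveals its death message after running parent logic.
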(event `self.ShootingComponent.OnAmmoChanged`
  (params (NewAmmo :type Integer))
  (bind _hud (`self.HUD`))
  (`/Engine/EditorBlueprintResources/StandardMacros.IsValid` _hud
    (:`Is Valid`
      (`/Game/UI/UI_HUD.SetAmmo` _hud NewAmmo))))

(event `self.OnHealthChanged`
  (params (HP :type "Float (single-precision)"))
  (bind _hud (`self.HUD`))
  (`/Engine/EditorBlueprintResources/StandardMacros.IsValid` _hud
    (:`Is Valid`
      (`/Game/UI/UI_HUD.SetHP` _hud HP))))

(event `self.ReceiveBeginPlay`
  (`parent.ReceiveBeginPlay`)
  (`WidgetLayoutLibrary.RemoveAllWidgets`)
  (bind _returnvalue (`|CreateWidget` "/Game/UI/UI_HUD.UI_HUD_C" (`GameplayStatics.GetPlayerController` 0)))
  (bind _output_get (set `self.HUD` _returnvalue))
  (`UserWidget.AddToViewport` _output_get 0)
  (`/Game/UI/UI_HUD.SetAmmo` _output_get (`ShootingComponent.GetCurrentAmmo` (`self.ShootingComponent`))))

(event `self.OnDeath`
  (`parent.OnDeath`)
  (`/Game/UI/UI_HUD.SetDeathMessageVisibility` (`self.HUD`) true))

(fn `UserConstructionScript`)