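; Gun turret pawn Blueprint that drives a skeletal railgun mesh through its animation Blueprint.
; A rotation event passes yaw and pitch to the anim BP as horizontal and vertical rotation.
; The Shoot override calls the parent, then on success spawns a half-scale explosion emitter at the barrel socket and triggers the anim BP's shoot.
; A failed anim BP cast prints an error.
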(event `self.RotateSkeletalGunMesh`
  (params (Yaw :type "Float (single-precision)") (Pitch :type "Float (single-precision)"))
  (bind _assk_rail_gun_anim_bp (cast `/Game/Assets/Models/SK_RailGunAnimBP` (`SkeletalMeshComponent.GetAnimInstance` (`self.GunMesh`)))
    (:`then`
      (set `/Game/Assets/Models/SK_RailGunAnimBP.HorizontalRotation` Yaw _assk_rail_gun_anim_bp)
      (set `/Game/Assets/Models/SK_RailGunAnimBP.VerticalRotation` Pitch _assk_rail_gun_anim_bp))
    (:`CastFailed`
      (`KismetSystemLibrary.PrintString` "ERROR: Can't access animation BP"))))

(fn `Shoot`
  (returns (ReturnValue :type Boolean))
  (bind _returnvalue (`parent.Shoot`))
  (if _returnvalue
    (`GameplayStatics.SpawnEmitterAttached` "/Game/StarterContent/Particles/P_Explosion.P_Explosion" (`self.GunMesh`) "barrel" (0.0 0.0 0.0) (struct) (0.5 0.5 0.5))
    (bind _assk_rail_gun_anim_bp (cast `/Game/Assets/Models/SK_RailGunAnimBP` (`SkeletalMeshComponent.GetAnimInstance` (`self.GunMesh`)))
      (:`then`
        (`/Game/Assets/Models/SK_RailGunAnimBP.Shoot` _assk_rail_gun_anim_bp))
      (:`CastFailed`
        (`KismetSystemLibrary.PrintString` "ERROR: Can't access animation BP")))
    (return _returnvalue)))

(fn `UserConstructionScript`)